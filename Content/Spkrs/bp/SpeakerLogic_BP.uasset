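; Speaker product configurator logic that cycles cabinet, speaker, accent and screen options across a list of speaker actors and shows the choices and price on a HUD.
; Each click handler advances a wrapping index, swaps materials or sets the screen Color parameter, then reads that index's data table row.
; Those rows feed one HUD refresh of descriptions and USD-formatted prices with a total.
; PlayAudio separately switches the music track.
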(event EventBeginPlay)

(event Collision|EventActorBeginOverlap
  (params (OtherActor :type Actor%20Object%20Reference)))

(event EventTick
  (params (DeltaSeconds :type Float%20%28single-precision%29)))

(fn ConstructionScript)

(fn CabinetClicked
  (bind _output_get (Variables|Default|SetCabinetIndex (Math|Integer|%(Integer) (+ (Variables|Default|GetCabinetIndex) 1) (Variables|Default|GetCabinetIndexMax))))
  (switch int _output_get
    (:0
      (CallFunction|SetCabinetMaterial "/Game/Spkrs/m/BlkGld_Cab.BlkGld_Cab"))
    (:1
      (CallFunction|SetCabinetMaterial "/Game/Spkrs/m/EbStl_Cab.EbStl_Cab"))
    (:2
      (CallFunction|SetCabinetMaterial "/Game/Spkrs/m/TkBlk_Cab.TkBlk_Cab"))
    (:3
      (CallFunction|SetCabinetMaterial "/Game/Spkrs/m/WalSlv_Cab.WalSlv_Cab"))
    (:4
      (CallFunction|SetCabinetMaterial "/Game/Spkrs/m/WhtCp_Cab.WhtCp_Cab")))
  (CallFunction|DisplayCabinetData (Variables|Default|GetCabinetIndex)))

(fn SetCabinetMaterial
  (params (Material :type Material%20Object%20Reference))
  (for _array_element (Variables|Default|GetSpeakerList)
    (bind _cabinetmesh (Default|GetCabinetComponent _array_element))
    (Rendering|Material|SetMaterial _cabinetmesh 0 Material)))

(fn InitializeSpeakerLogic
  (params (SpeakerList :type Array%20of%20Speaker%20BP%20Object%20References) (HUD :type HUD%20UI%20Object%20Reference))
  (Utilities|FlowControl|Sequence
    (:then_0
      ;[1 1 1] Store Speaker List reference for use in speaker logic bp
      (Variables|Default|SetSpeakerList SpeakerList))
    (:then_1
      ;[1 1 1] Store HUD reference for use in speaker logic bp
      (Variables|Default|SetHUD HUD))
    (:then_2
      ;[1 1 1] Initialize default HUD data on start
      (CallFunction|DisplayCabinetData)
      (CallFunction|DisplaySpeakerData)
      (CallFunction|DisplayAccentData)
      (CallFunction|DisplayScreenData))))

(fn SpeakerClicked
  (bind _output_get (Variables|Default|SetSpeakerIndex (Math|Integer|%(Integer) (+ (Variables|Default|GetSpeakerIndex) 1) (Variables|Default|GetSpeakerIndexMax))))
  (switch int _output_get
    (:0
      (CallFunction|SetSpeakerMaterials "/Game/Spkrs/m/BlkGld_Twt.BlkGld_Twt" "/Game/Spkrs/m/BlkGld_Wof.BlkGld_Wof"))
    (:1
      (CallFunction|SetSpeakerMaterials "/Game/Spkrs/m/TkBlk_Twt.TkBlk_Twt" "/Game/Spkrs/m/TkBlk_Wof.TkBlk_Wof"))
    (:2
      (CallFunction|SetSpeakerMaterials "/Game/Spkrs/m/WalSlv_Twt.WalSlv_Twt" "/Game/Spkrs/m/WalSlv_Wof.WalSlv_Wof"))
    (:3
      (CallFunction|SetSpeakerMaterials "/Game/Spkrs/m/WhtCp_Twt.WhtCp_Twt" "/Game/Spkrs/m/WhtCp_Wof.WhtCp_Wof")))
  (CallFunction|DisplaySpeakerData (Variables|Default|GetSpeakerIndex)))

(fn SetSpeakerMaterials
  (params (HornTweeterMaterial :type Material%20Object%20Reference) (WooferMaterial :type Material%20Object%20Reference))
  (for _array_element (Variables|Default|GetSpeakerList)
    (bind (_woofersmash _horntweetermash) (Default|GetSpeakerComponents _array_element))
    (Rendering|Material|SetMaterial _horntweetermash 0 HornTweeterMaterial)
    (Rendering|Material|SetMaterial _woofersmash 0 WooferMaterial)))

(fn SetAccentsMaterials
  (params (FootMaterial :type Material%20Object%20Reference) (AccentMaterial :type Material%20Object%20Reference))
  (for _array_element (Variables|Default|GetSpeakerList)
    (bind (_footmeshes _accentmeshes) (Default|GetAccentComponents _array_element))
    (Utilities|FlowControl|Sequence
      (:then_0
        (for _array_element_2 _footmeshes
          (Rendering|Material|SetMaterial _array_element_2 0 FootMaterial)))
      (:then_1
        (for _array_element_3 _accentmeshes
          (Rendering|Material|SetMaterial _array_element_3 0 AccentMaterial))))))

(fn AccentClicked
  (bind _output_get (Variables|Default|SetAccentIndex (Math|Integer|%(Integer) (+ (Variables|Default|GetAccentIndex) 1) (Variables|Default|GetAccentIndexMax))))
  (switch int _output_get
    (:0
      (CallFunction|SetAccentsMaterials "/Game/Spkrs/m/BlkGld_Ft.BlkGld_Ft" "/Game/Spkrs/m/BlkGld_Cab.BlkGld_Cab"))
    (:1
      (CallFunction|SetAccentsMaterials "/Game/Spkrs/m/EbStl_Ft.EbStl_Ft" "/Game/Spkrs/m/EbStl_Cab.EbStl_Cab"))
    (:2
      (CallFunction|SetAccentsMaterials "/Game/Spkrs/m/TkBlk_Ft.TkBlk_Ft" "/Game/Spkrs/m/TkBlk_Cab.TkBlk_Cab"))
    (:3
      (CallFunction|SetAccentsMaterials "/Game/Spkrs/m/WalSlv_Ft.WalSlv_Ft" "/Game/Spkrs/m/WalSlv_Cab.WalSlv_Cab"))
    (:4
      (CallFunction|SetAccentsMaterials "/Game/Spkrs/m/WhtCp_Ft.WhtCp_Ft" "/Game/Spkrs/m/WhtCp_Cab.WhtCp_Cab")))
  (CallFunction|DisplayAccentData (Variables|Default|GetAccentIndex)))

(fn SetScreenColor
  (params (ScreenColor :type Vector))
  (for _array_element (Variables|Default|GetSpeakerList)
    (bind _screenmesh (Default|GetScreenComponent _array_element))
    (Rendering|Material|SetVectorParameterValueonMaterials _screenmesh "Color" ScreenColor)))

(fn ScreenClicked
  (bind _output_get (Variables|Default|SetScreenIndex (Math|Integer|%(Integer) (+ (Variables|Default|GetScreenIndex) 1) (Variables|Default|GetScreenIndexMax))))
  (switch int _output_get
    (:0
      ;[0 0 0] Black
      (CallFunction|SetScreenColor "0, 0, 0"))
    (:1
      ;[0.1441 0.1155 0.0323] Gold
      (CallFunction|SetScreenColor "0.144100,0.115500,0.032300"))
    (:2
      ;[0.089 0.089 0.089] Dark Grey
      (CallFunction|SetScreenColor "0.089000,0.089000,0.089000"))
    (:3
      ;[1 1 1] White
      (CallFunction|SetScreenColor "1.000000,1.000000,1.000000"))
    (:4
      ;[0.0642 0.0237 0.0093] Dark Brown
      (CallFunction|SetScreenColor "0.064200,0.023700,0.009300")))
  (CallFunction|DisplayScreenData (Variables|Default|GetScreenIndex)))

(fn DisplayCabinetData
  (params (Index :type Integer))
  (bind _returnvalue (Utilities|GetDataTableRow "/Game/Data/Cabinette_Data.Cabinette_Data" (Utilities|String|StringToName (Utilities|String|ToString(Integer) Index)))
    (:then
      (Utilities|FlowControl|Sequence
        (:then_0
          (Variables|Default|SetCabinetShortDescription (.ShortDescription (Utilities|Struct|BreakSpeakerData_Structure _returnvalue))))
        (:then_1
          (Variables|Default|SetCabinetLongDescription (.LongDescription (Utilities|Struct|BreakSpeakerData_Structure _returnvalue))))
        (:then_2
          (Variables|Default|SetCabinetPrice (.Price (Utilities|Struct|BreakSpeakerData_Structure _returnvalue))))
        (:then_3
          (CallFunction|DisplayFinalDatatoHUD))))))

(fn DisplayFinalDatatoHUD
  (Utilities|FlowControl|Sequence
    (:then_0
      ;[1 1 1] Calc and set HUD TotalPrice
      (Variables|/Game/HUD/HUD_UI.HUD_UI_C|SetTotalPrice (Variables|Default|GetHUD) (CallFunction|PriceFormator (+ (Variables|Default|GetAccentPrice) (Variables|Default|GetScreenPrice) (Variables|Default|GetCabinetPrice) (Variables|Default|GetSpeakerPrice) (Variables|Default|GetBasePrice)))))
    (:then_1
      ;[1 1 1] Set HUD Prices
      (Variables|/Game/HUD/HUD_UI.HUD_UI_C|SetAccentPrice (Variables|Default|GetHUD) (CallFunction|PriceFormator (Variables|Default|GetAccentPrice)))
      (Variables|/Game/HUD/HUD_UI.HUD_UI_C|SetScreenPrice (Variables|Default|GetHUD) (CallFunction|PriceFormator (Variables|Default|GetScreenPrice)))
      (Variables|/Game/HUD/HUD_UI.HUD_UI_C|SetCabinetPrice (Variables|Default|GetHUD) (CallFunction|PriceFormator (Variables|Default|GetCabinetPrice)))
      (Variables|/Game/HUD/HUD_UI.HUD_UI_C|SetSpeakerPrice (Variables|Default|GetHUD) (CallFunction|PriceFormator (Variables|Default|GetSpeakerPrice)))
      (Variables|/Game/HUD/HUD_UI.HUD_UI_C|SetBasePrice (Variables|Default|GetHUD) (CallFunction|PriceFormator (Variables|Default|GetBasePrice))))
    (:then_2
      ;[1 1 1] Set HUD ShortDescription
      (Variables|/Game/HUD/HUD_UI.HUD_UI_C|SetAccentChoice (Variables|Default|GetHUD) (Variables|Default|GetAccentShortDescription))
      (Variables|/Game/HUD/HUD_UI.HUD_UI_C|SetScreenChoice (Variables|Default|GetHUD) (Variables|Default|GetScreenShortDescription))
      (Variables|/Game/HUD/HUD_UI.HUD_UI_C|SetCabinetChoice (Variables|Default|GetHUD) (Variables|Default|GetCabinetShortDescription))
      (Variables|/Game/HUD/HUD_UI.HUD_UI_C|SetSpeakerChoice (Variables|Default|GetHUD) (Variables|Default|GetSpeakerShortDescription)))
    (:then_3
      (Variables|/Game/HUD/HUD_UI.HUD_UI_C|SetSpeakersDescription (Variables|Default|GetHUD) (Utilities|Text|ToText(String) (Utilities|String|Append (Utilities|String|Append (Utilities|String|Append (Utilities|String|Append (Utilities|String|ToString(Text) (Variables|Default|GetSpeakerLongDescription)) "Speakers in") (Utilities|String|ToString(Text) (Variables|Default|GetCabinetLongDescription))) "Cabinet and") (Utilities|String|ToString(Text) (Variables|Default|GetAccentLongDescription))))))))

(fn DisplaySpeakerData
  (params (Index :type Integer))
  (bind _returnvalue (Utilities|GetDataTableRow "/Game/Data/Speaker_Data.Speaker_Data" (Utilities|String|StringToName (Utilities|String|ToString(Integer) Index)))
    (:then
      (Utilities|FlowControl|Sequence
        (:then_0
          (Variables|Default|SetSpeakerShortDescription (.ShortDescription (Utilities|Struct|BreakSpeakerData_Structure _returnvalue))))
        (:then_1
          (Variables|Default|SetSpeakerLongDescription (.LongDescription (Utilities|Struct|BreakSpeakerData_Structure _returnvalue))))
        (:then_2
          (Variables|Default|SetSpeakerPrice (.Price (Utilities|Struct|BreakSpeakerData_Structure _returnvalue))))
        (:then_3
          (CallFunction|DisplayFinalDatatoHUD))))))

(fn DisplayAccentData
  (params (Index :type Integer))
  (bind _returnvalue (Utilities|GetDataTableRow "/Game/Data/Accent_Data.Accent_Data" (Utilities|String|StringToName (Utilities|String|ToString(Integer) Index)))
    (:then
      (Utilities|FlowControl|Sequence
        (:then_0
          (Variables|Default|SetAccentShortDescription (.ShortDescription (Utilities|Struct|BreakSpeakerData_Structure _returnvalue))))
        (:then_1
          (Variables|Default|SetAccentLongDescription (.LongDescription (Utilities|Struct|BreakSpeakerData_Structure _returnvalue))))
        (:then_2
          (Variables|Default|SetAccentPrice (.Price (Utilities|Struct|BreakSpeakerData_Structure _returnvalue))))
        (:then_3
          (CallFunction|DisplayFinalDatatoHUD))))))

(fn DisplayScreenData
  (params (Index :type Integer))
  (bind _returnvalue (Utilities|GetDataTableRow "/Game/Data/Screen_Data.Screen_Data" (Utilities|String|StringToName (Utilities|String|ToString(Integer) Index)))
    (:then
      (Utilities|FlowControl|Sequence
        (:then_0
          (Variables|Default|SetScreenShortDescription (.ShortDescription (Utilities|Struct|BreakSpeakerData_Structure _returnvalue))))
        (:then_1
          (Variables|Default|SetScreenLongDescription (.LongDescription (Utilities|Struct|BreakSpeakerData_Structure _returnvalue))))
        (:then_2
          (Variables|Default|SetScreenPrice (.Price (Utilities|Struct|BreakSpeakerData_Structure _returnvalue))))
        (:then_3
          (CallFunction|DisplayFinalDatatoHUD))))))

(fn PriceFormator
  (params (PriceInCents :type Integer))
  (return (Class|KismetTextLibrary|AsCurrencyBase PriceInCents "USD")))

(fn PlayAudio
  (params (Track :type Integer))
  (Utilities|FlowControl|Sequence
    (:then_0
      ;[1 1 1] Stop the Audio Track
      (Audio|Components|Audio|Stop (Variables|Default|GetMusicComponent)))
    (:then_1
      ;[1 1 1] Load Audio Track
      (Audio|Components|Audio|SetSound (Variables|Default|GetMusicComponent) (Utilities|Array|Get(acopy) (Variables|Default|GetMusic_Tracks) Track)))
    (:then_2
      ;[1 1 1] Play Selected Audio Track
      (Audio|Components|Audio|Play (Variables|Default|GetMusicComponent) 0.0))))