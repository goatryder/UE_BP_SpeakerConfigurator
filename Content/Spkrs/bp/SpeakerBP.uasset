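; Clickable speaker actor built from separate meshes for cabinet, drivers, screen, feet and trim.
; Mesh clicks are grouped into accent, speaker, screen and cabinet categories and forwarded to a SpeakerLogicBP reference, while screw clicks do nothing.
; InitializeSpeakerBP stores that reference and applies the CoverActive flag, hiding Frame and Screen and ignoring their collision when inactive.
; Getter functions expose the meshes by category.
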(event OnClicked(Woofers)
  (params (TouchedComponent :type Primitive%20Component%20Object%20Reference) (ButtonPressed :type Key%20Structure :default "None"))
  ;[1 1 1] Speakers Clicked
  (Default|SpeakerClicked (Variables|Default|GetSpeakerLogicBPReference)))

(event OnClicked(HornTweeter)
  (params (TouchedComponent :type Primitive%20Component%20Object%20Reference) (ButtonPressed :type Key%20Structure :default "None"))
  ;[1 1 1] Speakers Clicked
  (Default|SpeakerClicked (Variables|Default|GetSpeakerLogicBPReference)))

(event OnClicked(Screws)
  (params (TouchedComponent :type Primitive%20Component%20Object%20Reference) (ButtonPressed :type Key%20Structure :default "None"))
  ;[1 1 1] Accents Clicked
)

(event OnClicked(AccentPlate)
  (params (TouchedComponent :type Primitive%20Component%20Object%20Reference) (ButtonPressed :type Key%20Structure :default "None"))
  ;[1 1 1] Accents Clicked
  (Default|AccentClicked (Variables|Default|GetSpeakerLogicBPReference)))

(event OnClicked(Cabinette)
  (params (TouchedComponent :type Primitive%20Component%20Object%20Reference) (ButtonPressed :type Key%20Structure :default "None"))
  ;[1 1 1] Cabinette Clicked
  (Default|CabinetClicked (Variables|Default|GetSpeakerLogicBPReference)))

(event OnClicked(Foot_BL)
  (params (TouchedComponent :type Primitive%20Component%20Object%20Reference) (ButtonPressed :type Key%20Structure :default "None"))
  ;[1 1 1] Accents Clicked
  (Default|AccentClicked (Variables|Default|GetSpeakerLogicBPReference)))

(event OnClicked(Foot_BR)
  (params (TouchedComponent :type Primitive%20Component%20Object%20Reference) (ButtonPressed :type Key%20Structure :default "None"))
  ;[1 1 1] Accents Clicked
  (Default|AccentClicked (Variables|Default|GetSpeakerLogicBPReference)))

(event OnClicked(Foot_FL)
  (params (TouchedComponent :type Primitive%20Component%20Object%20Reference) (ButtonPressed :type Key%20Structure :default "None"))
  ;[1 1 1] Accents Clicked
  (Default|AccentClicked (Variables|Default|GetSpeakerLogicBPReference)))

(event OnClicked(Foot_FR)
  (params (TouchedComponent :type Primitive%20Component%20Object%20Reference) (ButtonPressed :type Key%20Structure :default "None"))
  ;[1 1 1] Accents Clicked
  (Default|AccentClicked (Variables|Default|GetSpeakerLogicBPReference)))

(event OnClicked(Frame)
  (params (TouchedComponent :type Primitive%20Component%20Object%20Reference) (ButtonPressed :type Key%20Structure :default "None"))
  ;[1 1 1] Accents Clicked
  (Default|AccentClicked (Variables|Default|GetSpeakerLogicBPReference)))

(event OnClicked(Screen)
  (params (TouchedComponent :type Primitive%20Component%20Object%20Reference) (ButtonPressed :type Key%20Structure :default "None"))
  ;[1 1 1] Screen Clicked
  (Default|ScreenClicked (Variables|Default|GetSpeakerLogicBPReference)))

(event EventBeginPlay)

(event Collision|EventActorBeginOverlap
  (params (OtherActor :type Actor%20Object%20Reference)))

(event EventTick
  (params (DeltaSeconds :type Float%20%28single-precision%29)))

(fn ConstructionScript)

(fn GetCabinetComponent
  (return (Variables|Default|GetCabinette)))

(fn InitializeSpeakerBP
  (params (SpeakerLogicBP :type Speaker%20Logic%20BP%20Object%20Reference))
  (Utilities|FlowControl|Sequence
    (:then_0
      (Variables|Default|SetSpeakerLogicBPReference SpeakerLogicBP))
    (:then_1
      ;[1 1 1] Check cover active
      (if (Variables|Default|GetCoverActive)
        ;;[0.005822 1 0.0918] Cover is Active
        (Rendering|SetVisibility (Variables|Default|GetFrame) true false)
        (Rendering|SetVisibility (Variables|Default|GetScreen) true false)
        (else
          ;;[1 0.1455 0.2753] Cover is Inactive
          (Rendering|SetVisibility (Variables|Default|GetFrame) false false)
          (Rendering|SetVisibility (Variables|Default|GetScreen) false false)
          (Collision|SetCollisionResponsetoAllChannels (Variables|Default|GetFrame) "ECR_Ignore")
          (Collision|SetCollisionResponsetoAllChannels (Variables|Default|GetScreen) "ECR_Ignore"))))))

(fn GetSpeakerComponents
  (return (Variables|Default|GetWoofers) (Variables|Default|GetHornTweeter)))

(fn GetAccentComponents
  (return (Utilities|Array|MakeArray (Variables|Default|GetFoot_BR) (Variables|Default|GetFoot_FL) (Variables|Default|GetFoot_FR) (Variables|Default|GetFoot_BL)) (Utilities|Array|MakeArray (Variables|Default|GetFrame) (Variables|Default|GetAccentPlate))))

(fn GetScreenComponent
  (return (Variables|Default|GetScreen)))